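; BP_TagListner is a listener actor that waits on a gameplay tag check and is removed once it completes.
; On BeginPlay it runs GameTagCheckTool, a latent-style node with a Finished output, against the BP_TagChanger actor.
; When that finishes, it asks BP_MyPawn to despawn it through DespawnListnerSV, logging start and completion.
; Both actor references are found by GetActorOfClass and cached in getter functions.
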(event `self.ReceiveBeginPlay`
  (`GameTagCheckTool.GameTagCheckTool` (`self.GetTagChangerRef`)
    (:`then`
      (`KismetSystemLibrary.PrintString` "Started listening for tag"))
    (:`OnFinished`
      (`KismetSystemLibrary.PrintString` "Tag recieved - deleting listener" true true (struct :`R` 1.0 :`G` 0.036018 :`A` 1.0))
      (`/Game/Blueprints/Base/BP_MyPawn.DespawnListner_SV` (`self.GetPlayerRef`) self))
    (:`OnUpdated`)))

(fn `GetPlayerRef`
  (returns (MyPlayerRef :type "/Game/Blueprints/Base/BP_MyPawn Object Reference"))
  (bind _myplayerref (`self.MyPlayerRef`))
  (`/Engine/EditorBlueprintResources/StandardMacros.IsValid` _myplayerref
    (:`Is Valid`
      (return _myplayerref))
    (:`Is Not Valid`
      (bind _returnvalue (`GameplayStatics.GetActorOfClass` "/Game/Blueprints/Base/BP_MyPawn.BP_MyPawn_C"))
      (bind _output_get (set `self.MyPlayerRef` _returnvalue))
      (return _output_get))))

(fn `GetTagChangerRef`
  (returns (TagChangerRef :type "/Game/Blueprints/BP_TagChanger Object Reference"))
  (`/Engine/EditorBlueprintResources/StandardMacros.IsValid` (`self.TagChangerRef`)
    (:`Is Valid`
      (return (`self.TagChangerRef`)))
    (:`Is Not Valid`
      (bind _returnvalue (`GameplayStatics.GetActorOfClass` "/Game/Blueprints/BP_TagChanger.BP_TagChanger_C"))
      (bind _output_get (set `self.TagChangerRef` _returnvalue))
      (return _output_get))))

(fn `UserConstructionScript`)